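; BP_Loop is an actor Blueprint that builds a grid of static mesh components at BeginPlay, apparently as a loop exercise.
; An outer loop adds X-scaled meshes stepped along X, and a nested loop adds rotated, Y-scaled meshes across X and Y.
; Index counts, step spacing and scale come from variables.
; An unconnected loop that prints indices until a break never runs, and the construction script is empty.
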(event EventBeginPlay
  (bind _scale (Variables|Default|GetScale))
  (for _index (range 0 (Variables|Default|GetIndX))
    (AddComponent|AddStaticMeshComponent false (Math|Transform|MakeTransform (Math|Vector|MakeVector (* _index (Variables|Default|GetStepX)) 0.0 0.0) "0, 0, 0" (Math|Vector|MakeVector _scale 1.0 1.0)))
    (for _index_2 (range 0 (Variables|Default|GetIndY))
      (AddComponent|AddStaticMeshComponent false (Math|Transform|MakeTransform (Math|Vector|MakeVector (* _index (Variables|Default|GetStepX)) (* _index_2 (Variables|Default|GetStepY)) 0.0) "0,90.000000, 0" (Math|Vector|MakeVector 1.0 _scale 1.0))))))

(fn ConstructionScript)