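; BP_3DPriter is a 3D printer actor that spawns a requested number of Grabbable_SmallCube actors.
; The PrintButtonPressed event stores the count and spawns all the cubes in a single loop, with no delay between them.
; Cubes form a row along world X from the root component's location, spaced by Pacing and shifted by Offset, regardless of the printer's rotation.
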(event EventPrintButtonPressed
  (params (Numbber_of_Prints_I :type Integer))
  (bind _defaultsceneroot (Variables|Default|GetDefaultSceneRoot))
  (bind _returnvalue (Transformation|GetWorldLocation _defaultsceneroot))
  (Variables|Default|SetNumber_of_Printf Numbber_of_Prints_I)
  (for _index (range 0 (- (Variables|Default|GetNumber_of_Printf) 1))
    (Game|SpawnActorfromClass "/Game/VRTemplate/Blueprints/Grabbable_SmallCube.Grabbable_SmallCube_C" (Math|Transform|MakeTransform (Math|Vector|MakeVector (+ (.x _returnvalue) (* _index (Variables|Default|GetPacing)) (Variables|Default|GetOffset)) (.y _returnvalue) (.z _returnvalue)) "0, 0, 0" "1,1,1") "Undefined" 0 0)))

(fn ConstructionScript)