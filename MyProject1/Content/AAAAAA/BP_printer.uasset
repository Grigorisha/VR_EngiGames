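; BP_printer is an actor that spawns a batch of Grabbable_SmallCube actors when its PrintStarted event fires.
; The event stores the requested print count and loops that many times, spawning one cube per index at the root component's world X and Z.
; Each cube's Y is the root's world Y multiplied by index, Spacing and Offset, so placement scales with world position and the first cube lands at Y zero.
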(event EventPrintStarted
  (params (number_of_printsI :type Integer))
  (bind _defaultsceneroot (Variables|Default|GetDefaultSceneRoot))
  (bind _returnvalue (Transformation|GetWorldLocation _defaultsceneroot))
  (Variables|Default|Setnumber_of_prints number_of_printsI)
  (for _index (range 0 (- (Variables|Default|Getnumber_of_prints) 1))
    (Game|SpawnActorfromClass "/Game/VRTemplate/Blueprints/Grabbable_SmallCube.Grabbable_SmallCube_C" (Math|Transform|MakeTransform (Math|Vector|MakeVector (.x _returnvalue) (* (.y _returnvalue) (* _index (Variables|Default|Getspacing)) (Variables|Default|Getoffset)) (.z _returnvalue)) "0, 0, 0" "1,1,1") "Undefined" 0 0)))

(fn ConstructionScript)