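; BP_Loop is an actor Blueprint that spawns static mesh components in a four-column grid at BeginPlay.
; A for loop sets X from index modulo 4 times XSpacing and Y from an accumulated YSpacing.
; YSpacing grows after every fourth index's mesh is placed, so that mesh lands on the previous row's Y.
; An unconnected loop-with-break prints indices and a completion message but never runs.
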(event EventBeginPlay
  (for _index (range 0 (Variables|Default|GetLast%20Index))
    (AddComponent|AddStaticMeshComponent false (Math|Transform|MakeTransform (Math|Vector|MakeVector (* (Math|Integer|%(Integer) _index 4) (Variables|Default|GetXSpacing)) (Variables|Default|GetYSpacing) 0.0) "0, 0, 0" "1,1,1"))
    (if (and (== (Math|Integer|%(Integer) _index 4) 0) (!= _index 0))
      (Variables|Default|SetYSpacing (+ (Variables|Default|GetYSpacing) 2e+02)))))

(fn ConstructionScript)