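; BP_Origin is a drone assembly base where parts brought into the left motor, right motor and battery slots get installed.
; Each slot's overlap event casts to BP_PrintedParts (motors) or BP_Electronics (battery) and checks its Spec.
; A match destroys the part and reveals that slot's mesh, with DoOnce gating each motor.
; A wrong Spec increments a shared ErrorCounter and prints the total in Russian.
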(event OnComponentBeginOverlap(RightMotor)
  (params (OverlappedComponent :type Primitive%20Component%20Object%20Reference) (OtherActor :type Actor%20Object%20Reference) (OtherComp :type Primitive%20Component%20Object%20Reference) (OtherBodyIndex :type Integer) (bFromSweep :type Boolean) (SweepResult :type Hit%20Result%20Structure%20%28by%20ref%29))
  (bind _asbp_printed_parts (Utilities|Casting|CastToBP_PrintedParts OtherActor))
  (if (== (Variables|/Game/my_content/DroneLogic/BP_PrintedParts.BP_PrintedParts_C|GetSpec _asbp_printed_parts) 2)
    (Utilities|FlowControl|DoOnce false
      (:Completed
        (Actor|DestroyActor _asbp_printed_parts)
        (Rendering|SetVisibility (Variables|Default|GetSM_RightMotor) true false)))
    (else
      (bind _output_get (Variables|Default|SetErrorCounter (+ (Variables|Default|GetErrorCounter) 1)))
      (Development|PrintString (Utilities|String|Append "Текущее количество ошибок" (Utilities|String|ToString(Integer) _output_get))))))

(event OnComponentBeginOverlap(LeftMotor)
  (params (OverlappedComponent :type Primitive%20Component%20Object%20Reference) (OtherActor :type Actor%20Object%20Reference) (OtherComp :type Primitive%20Component%20Object%20Reference) (OtherBodyIndex :type Integer) (bFromSweep :type Boolean) (SweepResult :type Hit%20Result%20Structure%20%28by%20ref%29))
  (bind _asbp_printed_parts (Utilities|Casting|CastToBP_PrintedParts OtherActor))
  (if (== (Variables|/Game/my_content/DroneLogic/BP_PrintedParts.BP_PrintedParts_C|GetSpec _asbp_printed_parts) 2)
    (Utilities|FlowControl|DoOnce false
      (:Completed
        (Actor|DestroyActor _asbp_printed_parts)
        (Rendering|SetVisibility (Variables|Default|GetSM_LeftMotor) true false)))
    (else
      (bind _output_get (Variables|Default|SetErrorCounter (+ (Variables|Default|GetErrorCounter) 1)))
      (Development|PrintString (Utilities|String|Append "Текущее количество ошибок" (Utilities|String|ToString(Integer) _output_get))))))

(event OnComponentBeginOverlap(Battery)
  (params (OverlappedComponent :type Primitive%20Component%20Object%20Reference) (OtherActor :type Actor%20Object%20Reference) (OtherComp :type Primitive%20Component%20Object%20Reference) (OtherBodyIndex :type Integer) (bFromSweep :type Boolean) (SweepResult :type Hit%20Result%20Structure%20%28by%20ref%29))
  (bind _asbp_electronics (Utilities|Casting|CastToBP_Electronics OtherActor))
  (if (== (Variables|/Game/my_content/DroneLogic/BP_Electronics.BP_Electronics_C|GetSpec _asbp_electronics) 1)
    (Actor|DestroyActor _asbp_electronics)
    (Rendering|SetVisibility (Variables|Default|GetSM_Battery) true false)
    (else
      (bind _output_get (Variables|Default|SetErrorCounter (+ (Variables|Default|GetErrorCounter) 1)))
      (Development|PrintString (Utilities|String|Append "Текущее количество ошибок" (Utilities|String|ToString(Integer) _output_get))))))

(fn ConstructionScript)